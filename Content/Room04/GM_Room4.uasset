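; Room 4 game mode running a book-matching task where the player finds same-label pairs across different shelves.
; On task start it shuffles books and labels, gives matching labels to pairs split by shelf, hides some leftovers and labels the rest uniquely.
; Clicks compare against the previous book: matches are hidden and count toward completion, while mismatches fail the attempt and vibrate the player character.
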(event `self.ReceiveBeginPlay`
  (`self.StartTask` 0.0))

(event `self.OnTaskStarted`
  (bind _outactors (`GameplayStatics.GetAllActorsOfClass` "/Game/Room04/BookAndCupe/Book.Book_C"))
  (`self.GenerateBooksPlacement` 0.1 0.2 _outactors))

(fn `DropBook`
  (params (Book :type "/Game/Room04/BookAndCupe/Book Object Reference"))
  (`self.SetActorHiddenInGame` Book true)
  (`self.SetActorEnableCollision` Book false))

(fn `GenerateBooksPlacement`
  (params (HiddenBooksPercent :type "Float (double-precision)") (UniqueBooksPercent :type "Float (double-precision)") (AllBooks :type "Array of /Game/Room04/BookAndCupe/Book Object Reference"))
  (locals (BooksCountToPlace :type Integer) (`1Shelf_Books` :type "Array of /Game/Room04/BookAndCupe/Book Object Reference") (`2Shelf_Books` :type "Array of /Game/Room04/BookAndCupe/Book Object Reference") (BooksCountToDrop :type Integer) (UniqueBooksCount :type Integer) (LastLabelIndex :type Integer) (OtherBooks :type "Array of /Game/Room04/BookAndCupe/Book Object Reference"))
  (bind _returnvalue (`KismetArrayLibrary.Array_Length` AllBooks))
  (bind _otherbooks (`local.OtherBooks`))
  (bind _lastlabelindex (`local.LastLabelIndex`))
  (bind _lastlabelindex_2 (`local.LastLabelIndex`))
  (bind _returnvalue_2 (/ (`self.BooksCountToFind`) 2))
  (bind _output (`|GetArrayItem` (`self.BookLabels`) _lastlabelindex))
  ;[1 1 1] Shuffle books and labels for them
  (`KismetArrayLibrary.Array_Shuffle` AllBooks)
  (`KismetArrayLibrary.Array_Shuffle` (`self.BookLabels`))
  ;[1 1 1] Calc books count to hide, to place and with unique labels
  (set `local.BooksCountToDrop` (`KismetMathLibrary.FTrunc` (* _returnvalue HiddenBooksPercent)))
  (set `local.UniqueBooksCount` (`KismetMathLibrary.FTrunc` (* _returnvalue UniqueBooksPercent)))
  (bind _output_get (set `self.BooksCountToFind` (- (`KismetArrayLibrary.Array_Length` (`local.AllBooks`)) (+ (`local.BooksCountToDrop`) (`local.UniqueBooksCount`)))))
  (if (not (== (mod _output_get 2) 0))
    (`/Engine/EditorBlueprintResources/StandardMacros.DecrementInt` (`self.BooksCountToFind`)
      (:`  `
        (`/Engine/EditorBlueprintResources/StandardMacros.IncrementInt` (`local.UniqueBooksCount`)
          (:`  `
            _)))))
  (if (< (+ (`local.UniqueBooksCount`) (/ (`self.BooksCountToFind`) 2)) (`KismetArrayLibrary.Array_Length` (`self.BookLabels`)))
    (set `local.LastLabelIndex` 0)
    ;[1 1 1] Sort books
    (for _array_element (`local.AllBooks`)
      (if (== (`/Game/Room04/BookAndCupe/Book.ShelfID` _array_element) 1)
        (if (< (`KismetArrayLibrary.Array_Length` (`local.1Shelf_Books`)) _returnvalue_2)
          (`KismetArrayLibrary.Array_Add` (`local.1Shelf_Books`) _array_element)
          (else
            (`KismetArrayLibrary.Array_Add` (`local.OtherBooks`) _array_element :!label _label)))
        (elif (< (`KismetArrayLibrary.Array_Length` (`local.2Shelf_Books`)) _returnvalue_2)
          (`KismetArrayLibrary.Array_Add` (`local.2Shelf_Books`) _array_element)
          (else
            (goto _label)))))
    ;[1 1 1] Place books to find
    (for (_array_element_2 _array_index) (`local.1Shelf_Books`)
      (`/Game/Room04/BookAndCupe/Book.SetImage` _array_element_2 _output _lastlabelindex)
      (`/Game/Room04/BookAndCupe/Book.SetImage` (`|GetArrayItem` (`local.2Shelf_Books`) _array_index) _output _lastlabelindex)
      (`/Engine/EditorBlueprintResources/StandardMacros.IncrementInt` (`local.LastLabelIndex`)))
    ;[1 1 1] Hide random books
    (for _ (range (+ (`KismetMathLibrary.Min` (`local.BooksCountToDrop`) (`KismetArrayLibrary.Array_Length` (`local.OtherBooks`))) 1))
      (`self.DropBook` (`|GetArrayItem` _otherbooks))
      (`KismetArrayLibrary.Array_Remove` _otherbooks))
    ;[1 1 1] Place books with unique labels
    (for _array_element_3 (`local.OtherBooks`)
      (`/Game/Room04/BookAndCupe/Book.SetImage` _array_element_3 (`|GetArrayItem` (`self.BookLabels`) _lastlabelindex_2) _lastlabelindex_2)
      (`/Engine/EditorBlueprintResources/StandardMacros.IncrementInt` (`local.LastLabelIndex`)))
    (else
      (`KismetSystemLibrary.PrintString` "Not enouth labels for books" true true (struct :`R` 1.0 :`G` 0.205828 :`B` 0.150079 :`A` 1.0) 10.0))))

(fn `OnBookClicked`
  (params (Book :type "/Game/Room04/BookAndCupe/Book Object Reference"))
  (locals (NewClickedBook :type "/Game/Room04/BookAndCupe/Book Object Reference"))
  (bind _lastclickedbook (`self.lastClickedBook`))
  (bind _newclickedbook (`local.NewClickedBook`))
  (set `local.NewClickedBook` null)
  (`/Engine/EditorBlueprintResources/StandardMacros.IsValid` (`self.lastClickedBook`)
    (:`Is Valid`
      ;[1 1 1] Compare book labels
      (if (and (== (`/Game/Room04/BookAndCupe/Book.ImageID` _lastclickedbook) (`/Game/Room04/BookAndCupe/Book.ImageID` _newclickedbook)) (!= (`/Game/Room04/BookAndCupe/Book.ShelfID` _lastclickedbook) (`/Game/Room04/BookAndCupe/Book.ShelfID` _newclickedbook)))
        ;[1 1 1] Books are correct. Hide books
        (`self.DropBook` (`self.lastClickedBook`))
        (`self.DropBook` (`local.NewClickedBook`))
        (bind _result (`/Engine/EditorBlueprintResources/StandardMacros.DecrementInt` (`self.BooksCountToFind`))
          (:`  `
            (`/Engine/EditorBlueprintResources/StandardMacros.DecrementInt` _result
              (:`  `
                (`self.TryFinishTask`)))))
        (else
          (`self.FailAttempt`)
          ;[1 1 1] Wrong book clicked
          (bind _output_get (set `self.lastClickedBook` null))
          (set `local.NewClickedBook` _output_get)
          (bind _asinfromant (cast `/Game/Infromant` (`GameplayStatics.GetPlayerCharacter` 0)))
          (`BaseInformant.Vibrate` _asinfromant 1.0))))
    (:`Is Not Valid`
      ;[1 1 1] First book clicked
      (set `self.lastClickedBook` (`local.NewClickedBook`)))))

(fn `TryFinishTask`
  (if (== (`self.BooksCountToFind`) 0)
    (`self.FinishTask` 0)))

(fn `UserConstructionScript`)