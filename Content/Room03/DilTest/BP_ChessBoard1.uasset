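; Chessboard actor for a drag-and-drop figure puzzle in Room 3.
; On BeginPlay, 64Zone spawns one row of eight BoxCollisionPushBoard zones stepped along X from the Cone, despite its name, and a loop records the figure index.
; Disconnected logic spawns random draggable figures on the board, each scaled to cell size, given a trigger-box destination on a random free cell and shown as a GM_Room3 screen icon.
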(event `self.ReceiveBeginPlay`
  (`self.64Zone`)
  (for _index (range (+ (`self.QuantityFigure`) 1))
    (set `self.IndexQuantityFigure` _index)))

(fn `64Zone`
  (for _index (range 8)
    (bind _newparam (`self.CreateSizeZones` _index))
    (`|SpawnActorFromClass` "/Game/Room03/DilTest/BoxCollisionPushBoard.BoxCollisionPushBoard_C" _newparam "Undefined" "OverrideRootScale" null null))
  (set `self.StepNextZone` 0.0)
  (bind _result (`/Engine/EditorBlueprintResources/StandardMacros.IncrementFloat` (`self.StepY`))
    (:`  `
      (set `self.StepY` _result))))

(fn `completionCreateFigure`)

(fn `CreateSizeZones`
  (params (IndexNumZone :type Integer))
  (returns (NewParam :type "Transform Structure"))
  (set `self.StepNextZone` (* IndexNumZone (`self.StepX`)))
  (return (`KismetMathLibrary.MakeTransform` (`KismetMathLibrary.MakeVector` (+ (.x (.location (`SceneComponent.K2_GetComponentToWorld` (`self.Cone`)))) (`self.StepNextZone`)) (+ (.y (.location (`SceneComponent.K2_GetComponentToWorld` (`self.Cone`)))) (`self.StepY`)) (.z (.location (`SceneComponent.K2_GetComponentToWorld` (`self.Cone`))))) (.rotation (`SceneComponent.K2_GetComponentToWorld` (`self.Cone`))) (.scale (`SceneComponent.K2_GetComponentToWorld` (`self.Cone`))))))

(fn `RandomCell`
  (returns (Transform :type "Transform Structure") (CellWidth :type "Float (double-precision)") (RowIndex :type Integer) (ColumnIndex :type Integer))
  (locals (CellSize :type "Vector Structure"))
  (bind _freecells (`self.FreeCells`))
  (bind _cellsize (`local.CellSize`))
  (bind (_outitem _outindex) (`KismetArrayLibrary.Array_Random` _freecells))
  (bind _returnvalue (`KismetArrayLibrary.Array_LastIndex` _freecells))
  (bind (_min _max) (`StaticMeshComponent.GetLocalBounds` (`self.board`)))
  (bind _returnvalue_2 (/ _outitem 8))
  (bind _returnvalue_3 (mod _outitem 8))
  ;[1 1 1] Calc cell size
  (set `local.CellSize` (/ (- _max _min) 8.0))
  ;[1 1 1] Select random item and remove it from array
  (`KismetArrayLibrary.Array_Swap` _freecells _outindex _returnvalue)
  (`KismetArrayLibrary.Array_Remove` _freecells _returnvalue)
  (return (`KismetMathLibrary.ComposeTransforms` (`KismetMathLibrary.MakeTransform` (+ (* _cellsize (`KismetMathLibrary.MakeVector` (`KismetMathLibrary.Conv_IntToDouble` (- _returnvalue_2 4)) (`KismetMathLibrary.Conv_IntToDouble` (- _returnvalue_3 4)))) (/ _cellsize 2.0))) (`SceneComponent.K2_GetComponentToWorld` (`self.board`))) (.x (`local.CellSize`)) _returnvalue_3 _returnvalue_2))

(fn `RandomPosition`
  (params (Padding :type "Float (double-precision)"))
  (returns (Transform :type "Transform Structure"))
  (bind _returnvalue (`KismetMathLibrary.MakeVector` Padding Padding))
  (bind _board (`self.board`))
  (bind (_min _max) (`StaticMeshComponent.GetLocalBounds` _board))
  (return (`KismetMathLibrary.ComposeTransforms` (`KismetMathLibrary.MakeTransform` (`KismetMathLibrary.MakeVector` (`KismetMathLibrary.RandomFloatInRange` (.x (+ _returnvalue _min)) (.x (- _max _returnvalue))) (`KismetMathLibrary.RandomFloatInRange` (.y (+ _returnvalue _min)) (.y (- _max _returnvalue))))) (`SceneComponent.K2_GetComponentToWorld` _board))))

(fn `SpawnRandomFigure`
  ;[1 1 1] Spawn Trigger Destination
  (bind (_transform _cellwidth _rowindex _columnindex) (`self.RandomCell`))
  (bind _returnvalue (`|SpawnActorFromClass` "/Script/Engine.TriggerBox" _transform "Undefined" "OverrideRootScale" null null))
  (`KismetArrayLibrary.Array_Add` (`self.SpawnedTriggers`) _returnvalue)
  ;[1 1 1] Spawn Figure
  (bind _transform_2 (`self.RandomPosition` 10.0))
  (bind _returnvalue_2 (`|SpawnActorFromClass` (`KismetArrayLibrary.Array_Random` (`self.FigureClasses`)) _transform_2 "Undefined" "OverrideRootScale" null null))
  (`self.SetActorScale3D` _returnvalue_2 (`KismetMathLibrary.Conv_DoubleToVector` (/ _cellwidth 100.0)))
  (set `InteractableActor.bIsDraggable` true _returnvalue_2)
  (set `InteractableActor.DragAndDropDestination` _returnvalue _returnvalue_2)
  ;[1 1 1] Draw Icon on screen
  (bind _asgm_room_3 (cast `/Game/Room03/GM_Room3` (`GameplayStatics.GetGameMode`)))
  (bind _screen (`/Game/Room03/GM_Room3.Screen` _asgm_room_3))
  (`/Engine/EditorBlueprintResources/StandardMacros.IsValid` _screen
    (:`Is Valid`
      (`/Game/Room03/BP_ChessBoardScreen.AddFigureIcon` _screen _rowindex _columnindex (`/Game/Room03/Figure/BP_FigurePawn.Icon` _returnvalue_2)))
    (:`Is Not Valid`
      (`KismetSystemLibrary.PrintString` "Hello"))))

(fn `UserConstructionScript`)