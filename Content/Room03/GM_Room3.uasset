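; GM_Room3 is the game mode for Room 3, which starts the room's task once its key objects exist.
; Each tick, until the task has started, it waits for both the Board and Screen references to be valid, then calls StartTask and latches a flag.
; When the task starts, it forwards the event to the Board.
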(event `self.ReceiveTick`
  (params (DeltaSeconds :type "Float (single-precision)"))
  (if (not (`self.isTaskStarted`))
    (`/Engine/EditorBlueprintResources/StandardMacros.IsValid` (`self.Board`)
      (:`Is Valid`
        (`/Engine/EditorBlueprintResources/StandardMacros.IsValid` (`self.Screen`)
          (:`Is Valid`
            (`self.StartTask` 0.0)
            (set `self.isTaskStarted` true)))))))

(event `self.OnTaskStarted`
  (`/Game/Room03/ChessBoard/BP_ChessBoard.OnTaskStarted` (`self.Board`)))

(fn `UserConstructionScript`)