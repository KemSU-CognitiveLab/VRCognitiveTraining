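; Game mode for Room 1 that runs a colour-coded password puzzle, starting the task on BeginPlay.
; When the task starts, it picks and prints a random password, then generates an encoding using a set colour count per symbol.
; It passes both to the password panel.
; It then fills the encoding panel, mapping each character of a symbol's code to a colour through a lookup table.
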(event `self.ReceiveBeginPlay`
  (`self.StartTask` 0.0))

(event `self.OnTaskStarted`
  (bind _passwordpanel (`self.PasswordPanel`))
  (bind _encodingpanel (`self.EncodingPanel`))
  (`self.GenerateNewPassword`)
  (`/Engine/EditorBlueprintResources/StandardMacros.IsValid` _passwordpanel
    (:`Is Valid`
      (`/Game/Room01/PasswordPanel_Actor.SetPassword` _passwordpanel (`self.CurrentPassword`))
      (`/Game/Room01/PasswordPanel_Actor.SetEncoding` _passwordpanel (`self.CurrentEncoding`))
      (`/Engine/EditorBlueprintResources/StandardMacros.IsValid` _encodingpanel
        (:`Is Valid`
          (`/Game/Room01/EncodingPaper_Actor.Clear` _encodingpanel)
          (`self.View Encoding on UI`))))))

(fn `GenerateNewPassword`
  (bind _currentpassword (`self.CurrentPassword`))
  ;[1 1 1] Create new password
  (set `self.CurrentPassword` (`KismetArrayLibrary.Array_Random` (`self.Passwords`)))
  (`KismetSystemLibrary.PrintString` _currentpassword)
  ;[1 1 1] Generate encoding
  (bind _returnvalue (`CognitiveTrainingUtils.GenerateEncoding` _currentpassword (`self.ColorsCountPerSymbol`)))
  (set `self.CurrentEncoding` _returnvalue))

(fn `UserConstructionScript`)

(fn `View Encoding on UI`
  (locals (ColorsForSpell :type "Array of Color Structure"))
  (bind _currentencoding (`self.CurrentEncoding`))
  (bind _keys (`BlueprintMapLibrary.Map_Keys` _currentencoding))
  (for _array_element _keys
    (bind _returnvalue (`CognitiveTrainingUtils.BreakWordIntoCharacters` (`BlueprintMapLibrary.Map_Find` _currentencoding _array_element) true))
    (`KismetArrayLibrary.Array_Clear` (`local.ColorsForSpell`))
    (for _array_element_2 _returnvalue
      (`KismetArrayLibrary.Array_Add` (`local.ColorsForSpell`) (`BlueprintMapLibrary.Map_Find` (`self.Colors`) _array_element_2)))
    (`/Game/Room01/EncodingPaper_Actor.AddSymbol` (`self.EncodingPanel`) _array_element (`local.ColorsForSpell`))))